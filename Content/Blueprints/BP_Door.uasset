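; BP_Door is an interactive door that the player opens and closes with the E key.
; Box overlap enables input for player 0 and shows a W_Interaction prompt, and end overlap reverses both, without checking which actor overlaps.
; E toggles DoorOpen and snaps the static mesh between two fixed world rotations, with no interpolation.
; Level Sequence nodes for a DoorOpening animation are present but never run.
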(event `Key|E`
  (params (Key :type "Key Structure"))
  (bind _staticmesh (`self.StaticMesh`))
  (:`Pressed`
    (if (`self.DoorOpen?`)
      (`SceneComponent.K2_SetWorldRotation` _staticmesh (struct) false false)
      (set `self.DoorOpen?` false)
      (else
        (`SceneComponent.K2_SetWorldRotation` _staticmesh (struct :`Yaw` 100.0) false false)
        (set `self.DoorOpen?` true)))))

(event `self.Box.OnComponentBeginOverlap`
  (params (OverlappedComponent :type "PrimitiveComponent Object Reference") (OtherActor :type "Actor Object Reference") (OtherComp :type "PrimitiveComponent Object Reference") (OtherBodyIndex :type Integer) (bFromSweep :type Boolean) (SweepResult :type "HitResult Structure (by ref)"))
  (`self.EnableInput` (`GameplayStatics.GetPlayerController` 0))
  (bind _returnvalue (`|CreateWidget` "/Game/Blueprints/Widgets/W_Interaction.W_Interaction_C"))
  (`UserWidget.AddToViewport` _returnvalue 0))

(event `self.Box.OnComponentEndOverlap`
  (params (OverlappedComponent :type "PrimitiveComponent Object Reference") (OtherActor :type "Actor Object Reference") (OtherComp :type "PrimitiveComponent Object Reference") (OtherBodyIndex :type Integer))
  (`self.DisableInput` (`GameplayStatics.GetPlayerController` 0))
  (`Widget.RemoveFromParent` (stale `self.Box.OnComponentBeginOverlap` _returnvalue)))

(fn `UserConstructionScript`)