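; BP_Fire is an interactable fire pickup that plays a looping Wwise fire sound from BeginPlay.
; Overlapping its box enables player input and shows a prompt widget; leaving disables input and removes the widget.
; Pressing E casts the actor from the begin-overlap event to ThirdPersonCharacter, sets HasFire, plays a pickup sound and destroys the fire.
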(event `self.ReceiveBeginPlay`
  (`AkGameplayStatics.PostEvent` "/Game/WwiseAudio/Events/Default_Work_Unit/Fire/FireLoop.FireLoop" (`self.ActorSound`)))

(event `Key|E`
  (params (Key :type "Key Structure"))
  (:`Pressed`
    (bind _asthird_person_character (cast `/Game/ThirdPersonBP/Blueprints/ThirdPersonCharacter` (stale `self.Box.OnComponentBeginOverlap` OtherActor)))
    (set `/Game/ThirdPersonBP/Blueprints/ThirdPersonCharacter.HasFire?` true _asthird_person_character)
    (`AkGameplayStatics.PostEvent` "/Game/WwiseAudio/Events/Default_Work_Unit/Fire/FirePickUp.FirePickUp" (`self.ActorSound`) 1)
    (`self.K2_DestroyActor`)))

(event `self.Box.OnComponentBeginOverlap`
  (params (OverlappedComponent :type "PrimitiveComponent Object Reference") (OtherActor :type "Actor Object Reference") (OtherComp :type "PrimitiveComponent Object Reference") (OtherBodyIndex :type Integer) (bFromSweep :type Boolean) (SweepResult :type "HitResult Structure (by ref)"))
  ;[1 1 1] Print Interaction Widget on screen & Enable Player Input
  (`self.EnableInput` (`GameplayStatics.GetPlayerController` 0))
  (set `self.Player Is in Trigger` true)
  (bind _returnvalue (`|CreateWidget` (`self.Widget`)))
  (`UserWidget.AddToViewport` _returnvalue 0))

(event `self.Box.OnComponentEndOverlap`
  (params (OverlappedComponent :type "PrimitiveComponent Object Reference") (OtherActor :type "Actor Object Reference") (OtherComp :type "PrimitiveComponent Object Reference") (OtherBodyIndex :type Integer))
  ;[1 1 1] Print Interaction Widget on screen & Enable Player Input
  (`self.DisableInput` (`GameplayStatics.GetPlayerController` 0) null)
  (set `self.Player Is in Trigger` false)
  (if (not (`self.Player Is in Trigger`))
    (`Widget.RemoveFromParent` (stale `self.Box.OnComponentBeginOverlap` _returnvalue))))

(fn `UserConstructionScript`)