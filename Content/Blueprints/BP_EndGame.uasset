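; BP_EndGame is a trigger volume that ends the game when the third-person character enters its box.
; On overlap it disables the character's movement and plays the EndGame level sequence as a cutscene.
; It posts Wwise narration and fade-out events on the character.
; The narration event's callback waits briefly, then quits the game.
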(event `self.Box.OnComponentBeginOverlap`
  (params (OverlappedComponent :type "PrimitiveComponent Object Reference") (OtherActor :type "Actor Object Reference") (OtherComp :type "PrimitiveComponent Object Reference") (OtherBodyIndex :type Integer) (bFromSweep :type Boolean) (SweepResult :type "HitResult Structure (by ref)"))
  (bind _asthird_person_character (cast `/Game/ThirdPersonBP/Blueprints/ThirdPersonCharacter` OtherActor))
  (bind _output_get (set `self.TPC` _asthird_person_character))
  (`CharacterMovementComponent.DisableMovement` (`Character.CharacterMovement` _output_get))
  (bind (_outactor _returnvalue) (`LevelSequencePlayer.CreateLevelSequencePlayer` "/Game/Cutscenes/EndGame.EndGame"))
  (set `self.Cutscene` _returnvalue)
  (`MovieSceneSequencePlayer.Play` (`self.Cutscene`))
  (`AkGameplayStatics.PostEvent` (`self.Narrators Take`) (`self.TPC`) 1 (delegate `End Play`))
  (`AkGameplayStatics.PostEvent` "/Game/WwiseAudio/Events/Default_Work_Unit/Fades/FadeOutEnd.FadeOutEnd" (`self.TPC`)))

(event `End Play`
  (params (CallbackType :type "EAkCallbackType Enum" :default "EndOfEvent") (CallbackInfo :type "AkCallbackInfo Object Reference"))
  (`KismetSystemLibrary.Delay` 3.0)
  (`KismetSystemLibrary.QuitGame` null "Quit"))

(fn `UserConstructionScript`)