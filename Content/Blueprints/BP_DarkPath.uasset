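; BP_DarkPath is a one-shot interaction trigger that plays the NAR_03 narration through Wwise.
; Entering the trigger shows a prompt widget and enables input, or destroys the actor if the player already has the flashback.
; Pressing E removes the prompt, disables input and posts the event on the player character.
; The character's IsSoundPlaying flag blocks overlapping sounds and is cleared by the Wwise callback.
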(event `Key|E`
  (params (Key :type "Key Structure"))
  (:`Pressed`
    (if (`/Game/ThirdPersonBP/Blueprints/ThirdPersonCharacter.IsSoundPlaying` (`self.TPC`))
      _
      (elif (`self.FirstPlay?`)
        (set `self.FirstPlay?` false)
        (`self.DisableInput` (`GameplayStatics.GetPlayerController` 0))
        (`Widget.RemoveFromParent` (`self.UserWidget`))
        (`AkGameplayStatics.PostEvent` "/Game/WwiseAudio/Events/Voices/NAR_03.NAR_03" (`GameplayStatics.GetPlayerCharacter` 0) 1 (delegate `CustomEvent_0`))
        (set `/Game/ThirdPersonBP/Blueprints/ThirdPersonCharacter.IsSoundPlaying` true (`self.TPC`))))))

(event `CustomEvent_0`
  (params (CallbackType :type "EAkCallbackType Enum" :default "EndOfEvent") (CallbackInfo :type "AkCallbackInfo Object Reference"))
  (set `/Game/ThirdPersonBP/Blueprints/ThirdPersonCharacter.IsSoundPlaying` false (`self.TPC`)))

(event `self.Trigger.OnComponentBeginOverlap`
  (params (OverlappedComponent :type "PrimitiveComponent Object Reference") (OtherActor :type "Actor Object Reference") (OtherComp :type "PrimitiveComponent Object Reference") (OtherBodyIndex :type Integer) (bFromSweep :type Boolean) (SweepResult :type "HitResult Structure (by ref)"))
  (bind _asthird_person_character (cast `/Game/ThirdPersonBP/Blueprints/ThirdPersonCharacter` OtherActor))
  (bind _output_get (set `self.TPC` _asthird_person_character))
  (if (`/Game/ThirdPersonBP/Blueprints/ThirdPersonCharacter.HasFlashback?` _output_get)
    (`self.K2_DestroyActor`)
    (elif (`self.FirstPlay?`)
      (bind _returnvalue (`|CreateWidget` (`self.Widget`)))
      (bind _output_get_2 (set `self.UserWidget` _returnvalue))
      (`UserWidget.AddToViewport` _output_get_2 0)
      (`self.EnableInput` (`GameplayStatics.GetPlayerController` 0)))))

(event `self.Trigger.OnComponentEndOverlap`
  (params (OverlappedComponent :type "PrimitiveComponent Object Reference") (OtherActor :type "Actor Object Reference") (OtherComp :type "PrimitiveComponent Object Reference") (OtherBodyIndex :type Integer))
  (`self.DisableInput` (`GameplayStatics.GetPlayerController` 0))
  (`Widget.RemoveFromParent` (`self.UserWidget`)))

(fn `UserConstructionScript`)