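; BP_NarratorVoice is an interactable trigger that plays a narrator Wwise event when the player presses E nearby.
; Overlap by the third-person character enables input and prints a prompt, and any end overlap disables input.
; Pressing E posts NarratorsTake on the player character and prints a message, guarded by IsSoundPlaying, which is never reset here, so it fires only once.
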(event `Key|E`
  (params (Key :type "Key Structure"))
  ;[1 1 1] Player interaction and narrative/Sound
  (:`Pressed`
    (if (not (`self.IsSoundPlaying?`))
      (set `self.IsSoundPlaying?` true)
      (`AkGameplayStatics.PostEvent` (`self.Narrators Take`) (`GameplayStatics.GetPlayerCharacter` 0))
      (`KismetSystemLibrary.PrintString` "Hello"))))

(event `self.Trigger.OnComponentBeginOverlap`
  (params (OverlappedComponent :type "PrimitiveComponent Object Reference") (OtherActor :type "Actor Object Reference") (OtherComp :type "PrimitiveComponent Object Reference") (OtherBodyIndex :type Integer) (bFromSweep :type Boolean) (SweepResult :type "HitResult Structure (by ref)"))
  ;[1 1 1] Enable Player Input
  (cast `/Game/ThirdPersonBP/Blueprints/ThirdPersonCharacter` OtherActor)
  (`self.EnableInput` (`GameplayStatics.GetPlayerController` 0))
  (`KismetSystemLibrary.PrintString` "Press E to Interact"))

(event `self.Trigger.OnComponentEndOverlap`
  (params (OverlappedComponent :type "PrimitiveComponent Object Reference") (OtherActor :type "Actor Object Reference") (OtherComp :type "PrimitiveComponent Object Reference") (OtherBodyIndex :type Integer))
  ;[1 1 1] Enable Player Input
  (`self.DisableInput` (`GameplayStatics.GetPlayerController` 0)))

(fn `UserConstructionScript`)