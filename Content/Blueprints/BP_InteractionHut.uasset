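; BP_InteractionHut is an interactable hut prop that plays Wwise narrator audio when E is pressed inside its trigger.
; Trigger overlap enables input and shows a prompt widget, and leaving disables input and removes it.
; The E press casts the overlapping actor to ThirdPersonCharacter, using its IsSoundPlaying flag with a timed delay to block repeat playback.
; The construction script picks the mesh from an array by MeshChoise.
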(event `Key|E`
  (params (Key :type "Key Structure"))
  (:`Pressed`
    (bind _asthird_person_character (cast `/Game/ThirdPersonBP/Blueprints/ThirdPersonCharacter` (stale `self.Trigger.OnComponentBeginOverlap` OtherActor)))
    (if (not (`/Game/ThirdPersonBP/Blueprints/ThirdPersonCharacter.IsSoundPlaying` _asthird_person_character))
      (`AkGameplayStatics.PostEvent` (`self.Narrators Take`) (`GameplayStatics.GetPlayerCharacter` 0))
      (set `/Game/ThirdPersonBP/Blueprints/ThirdPersonCharacter.IsSoundPlaying` true _asthird_person_character)
      (`KismetSystemLibrary.Delay` (`self.Duration`))
      (set `/Game/ThirdPersonBP/Blueprints/ThirdPersonCharacter.IsSoundPlaying` false _asthird_person_character))))

(event `self.Trigger.OnComponentBeginOverlap`
  (params (OverlappedComponent :type "PrimitiveComponent Object Reference") (OtherActor :type "Actor Object Reference") (OtherComp :type "PrimitiveComponent Object Reference") (OtherBodyIndex :type Integer) (bFromSweep :type Boolean) (SweepResult :type "HitResult Structure (by ref)"))
  (`self.EnableInput` (`GameplayStatics.GetPlayerController` 0))
  (bind _returnvalue (`|CreateWidget` (`self.Widget`)))
  (`UserWidget.AddToViewport` _returnvalue 0))

(event `self.Trigger.OnComponentEndOverlap`
  (params (OverlappedComponent :type "PrimitiveComponent Object Reference") (OtherActor :type "Actor Object Reference") (OtherComp :type "PrimitiveComponent Object Reference") (OtherBodyIndex :type Integer))
  (`self.DisableInput` (`GameplayStatics.GetPlayerController` 0))
  (`self.DisableInput` null)
  (`Widget.RemoveFromParent` (stale `self.Trigger.OnComponentBeginOverlap` _returnvalue)))

(fn `UserConstructionScript`
  (locals (StaticMeshes :type "Array of StaticMesh Object Reference"))
  (`StaticMeshComponent.SetStaticMesh` (`self.Mesh`) (`|GetArrayItem` (`local.StaticMeshes`) (`KismetMathLibrary.Conv_ByteToInt` (`self.MeshChoise`)))))