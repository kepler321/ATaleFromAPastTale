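; Hide-and-seek trigger actor that plays a one-time Wwise audio sequence on the player character when overlapped.
; Any overlap fetches player 0's ThirdPersonCharacter and fires only if no sound is playing and HasFlashback is false.
; It sets the character's shared IsSoundPlaying lock, then chains NAR_05 into HNS_01 through end-of-event callbacks, releasing the lock when the second finishes.
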(event `self.ReceiveActorBeginOverlap`
  (params (OtherActor :type "Actor Object Reference"))
  (bind _asthird_person_character (cast `/Game/ThirdPersonBP/Blueprints/ThirdPersonCharacter` (`GameplayStatics.GetPlayerCharacter` 0)))
  (bind _output_get (set `self.TPC` _asthird_person_character))
  (if (`/Game/ThirdPersonBP/Blueprints/ThirdPersonCharacter.IsSoundPlaying` _output_get)
    _
    (elif (`self.FirstPlay?`)
      (if (not (`/Game/ThirdPersonBP/Blueprints/ThirdPersonCharacter.HasFlashback?` (`self.TPC`)))
        (set `self.FirstPlay?` false)
        (set `/Game/ThirdPersonBP/Blueprints/ThirdPersonCharacter.IsSoundPlaying` true (`self.TPC`))
        (`AkGameplayStatics.PostEvent` "/Game/WwiseAudio/Events/Voices/NAR_05.NAR_05" (`self.TPC`) 1 (delegate `End Play`))))))

(event `End Play`
  (params (CallbackType :type "EAkCallbackType Enum" :default "EndOfEvent") (CallbackInfo :type "AkCallbackInfo Object Reference"))
  (`AkGameplayStatics.PostEvent` "/Game/WwiseAudio/Events/Voices/HNS_01.HNS_01" (`self.TPC`) 1 (delegate `CustomEvent`)))

(event `self.ReceiveTick`
  (params (DeltaSeconds :type "Float (single-precision)")))

(event `CustomEvent`
  (params (CallbackType :type "EAkCallbackType Enum" :default "EndOfEvent") (CallbackInfo :type "AkCallbackInfo Object Reference"))
  (set `/Game/ThirdPersonBP/Blueprints/ThirdPersonCharacter.IsSoundPlaying` false (`self.TPC`)))

(fn `UserConstructionScript`)